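; Enemy AI Blueprint that patrols between two points and chases when its PawnSensing component sees a pawn.
; Patrolling loops AIMoveTo between the Start and Start0 actors, pausing briefly after each successful move.
; A sighting issues a move toward player controller 0 (not its pawn), then restarts patrol after a fixed delay, regardless of whether that move finishes.
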(event `self.ReceiveBeginPlay`
  (`self.Patroulieren`))

(event `self.PawnSensing.OnSeePawn`
  (params (Pawn :type "Pawn Object Reference"))
  (`self.Verfolgen`))

(event `Patroulieren`
  (`|AIMoveTo` self (0.0 0.0 0.0) (`self.Start`) 5.0 true
    (:`OnSuccess`
      (`KismetSystemLibrary.Delay` 1.0)
      (`|AIMoveTo` self (0.0 0.0 0.0) (`self.Start_0`) 5.0 true
        (:`OnSuccess`
          (`KismetSystemLibrary.Delay` 1.0)
          (`self.Patroulieren`))))))

(event `Verfolgen`
  (`|AIMoveTo` self (0.0 0.0 0.0) (`GameplayStatics.GetPlayerController` 0) 5.0 true
    (:`then`
      (`KismetSystemLibrary.Delay` 3.0)
      (`self.Patroulieren`))))

(fn `UserConstructionScript`)