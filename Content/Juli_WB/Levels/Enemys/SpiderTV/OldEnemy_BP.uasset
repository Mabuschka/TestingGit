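; An older SpiderTV enemy pawn that patrols between two actors and switches to a chase when it senses the player.
; Patrol loops AI move-to calls between Start and Start0 with two-second pauses.
; PawnSensing sight or hearing activates sparks and attached sound, then moves toward the player controller.
; As that move is issued, it destroys itself and the sound if the player character is within range.
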(event `self.ReceiveBeginPlay`
  (`self.Patroulieren`))

(event `self.PawnSensing.OnHearNoise`
  (params (Instigator :type "Pawn Object Reference") (Location :type "Vector Structure (by ref)") (Volume :type "Float (single-precision)"))
  (`self.Verfolgen` :!label _label))

(event `self.PawnSensing.OnSeePawn`
  (params (Pawn :type "Pawn Object Reference"))
  (goto _label))

(event `Patroulieren`
  (`|AIMoveTo` self (0.0 0.0 0.0) (`self.Start`) 5.0 true
    (:`OnSuccess`
      (`KismetSystemLibrary.Delay` 2.0)
      (`|AIMoveTo` self (0.0 0.0 0.0) (`self.Start_0`) 5.0 true
        (:`OnSuccess`
          (`KismetSystemLibrary.Delay` 2.0)
          (`self.Patroulieren`))))))

(event `Verfolgen`
  (`ActorComponent.SetActive` (`self.P_Sparks`) true false)
  (bind _returnvalue (`GameplayStatics.SpawnSoundAttached` "/Game/StarterContent/Audio/Fire_Sparks01_Cue.Fire_Sparks01_Cue" (`self.Mesh`) "None" (0.0 0.0 0.0) (struct) "KeepRelativeOffset" false 1.0 1.0 0.0 null null))
  (`|AIMoveTo` self (0.0 0.0 0.0) (`GameplayStatics.GetPlayerController` 0) 5.0 true
    (:`then`
      (if (<= (`self.GetDistanceTo` (`GameplayStatics.GetPlayerCharacter` 0) self) 300.0)
        (`ActorComponent.K2_DestroyComponent` _returnvalue)
        (`self.K2_DestroyActor`)))))

(fn `UserConstructionScript`)